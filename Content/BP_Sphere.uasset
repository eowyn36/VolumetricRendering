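; BP_Sphere is an actor that the player slides around with the arrow keys.
; It enables input on BeginPlay, and key events store the last pressed key and a shared IsPressed flag, which any arrow release clears.
; While the flag is set, Tick switches on the key's display name and applies a swept, fixed per-frame offset along the negated or positive right/forward vector, held in a variable misleadingly named Rotation.
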(event EventBeginPlay
  (Input|EnableInput (Game|GetPlayerController 0)))

(event EventTick
  (params (DeltaSeconds :type Float%20%28single-precision%29))
  (bind _returnvalue (Transformation|GetActorRightVector))
  (bind _returnvalue_2 (Transformation|GetActorForwardVector))
  (if (Variables|Default|GetisPressed)
    (switch string (Utilities|String|ToString(Text) (Class|KismetInputLibrary|KeyGetDisplayName (Variables|Default|GetpressedKey)))
      (:Right
        (Variables|Default|Setrotation (* _returnvalue -1e+01)))
      (:Left
        (Variables|Default|Setrotation (* _returnvalue 1e+01)))
      (:Up
        (Variables|Default|Setrotation (* _returnvalue_2 -1e+01)))
      (:Down
        (Variables|Default|Setrotation (* _returnvalue_2 1e+01))))
    (Transformation|SetActorLocation (+ (Transformation|GetActorLocation) (Variables|Default|Getrotation)) true false)))

(event Input|KeyboardEvents|Right
  (params (Key :type Key%20Structure :default "AnyKey"))
  (:Pressed
    (Variables|Default|SetpressedKey Key)
    (Variables|Default|SetisPressed true))
  (:Released
    (Variables|Default|SetisPressed false)))

(event Input|KeyboardEvents|Left
  (params (Key :type Key%20Structure :default "AnyKey"))
  (:Pressed
    (Variables|Default|SetpressedKey Key)
    (Variables|Default|SetisPressed true))
  (:Released
    (Variables|Default|SetisPressed false)))

(event Input|KeyboardEvents|Up
  (params (Key :type Key%20Structure :default "AnyKey"))
  (:Pressed
    (Variables|Default|SetpressedKey Key)
    (Variables|Default|SetisPressed true))
  (:Released
    (Variables|Default|SetisPressed false)))

(event Input|KeyboardEvents|Down
  (params (Key :type Key%20Structure :default "AnyKey"))
  (:Pressed
    (Variables|Default|SetpressedKey Key)
    (Variables|Default|SetisPressed true))
  (:Released
    (Variables|Default|SetisPressed false)))

(fn ConstructionScript)